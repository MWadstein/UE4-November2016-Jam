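; Finish platform that, when clicked, activates a particle effect and notifies the Game Mode, with a short timer lockout against repeat clicks.
; ToggleVisibility shows or hides the platform and switches its Visibility channel collision between Block and Ignore; that channel starts ignored at BeginPlay.
; Hovering plays a timeline that pulses emissive strength on three dynamic materials for the middle, left and right meshes.
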(event `/Game/Blueprints/Platforms/BPI_Platform.ToggleVisibility`
  (params (IsVisible :type Boolean) (CheatingTurnedOn :type Boolean))
  ;[1 1 1] Handle Toggling Visibility
  (`SceneComponent.SetVisibility` (`self.Platform`) IsVisible true) ; Set our New Visibility
  (`PrimitiveComponent.SetCollisionResponseToChannel` (`self.Platform`) "ECC_Visibility" (select `bool` IsVisible :`false` "ECR_Ignore" :`true` "ECR_Block" :!type "ECollisionResponse Enum")) ; Set our New Collision
)

(event `self.Platform.OnClicked`
  (params (TouchedComponent :type "PrimitiveComponent Object Reference") (ButtonPressed :type "Key Structure" :default "AnyKey"))
  ;[1 1 1] Handle being clicked on
  (if (not (`self.WasClickedOn`))
    (set `self.WasClickedOn` true)
    (`ActorComponent.SetActive` (`self.ParticleSystem`) true true) ; Turn on our particle system
    (message `/Game/Blueprints/Framework/BPI_LevelGameMode.FinishClickedOn` (`GameplayStatics.GetGameMode`) self) ; Tell the Game Mode we have been clicked on
    (`KismetSystemLibrary.K2_SetTimer` null "ResetWasClickedOn" 1.0) ; Allow ourself to be clicked on again in a second
  ))

(event `ResetWasClickedOn`
  ;[1 1 1] Allow ourself to be clicked on again
  (set `self.WasClickedOn` false))

(event `self.Platform.OnBeginCursorOver`
  (params (TouchedComponent :type "PrimitiveComponent Object Reference"))
  ;[1 1 1] Pulse when we are hovered
  (`self.PulseMaterial`))

(event `PulseMaterial`
  ;[1 1 1] Pulse all 3 of our Platform Objects
  (bind (_direction _0_10) (`Timeline|Timeline_0` :!via `PlayFromStart`)
    (:`Update`
      (`MaterialInstanceDynamic.SetScalarParameterValue` (`self.MiddlePlatform_MID`) "EmissiveStrength" _0_10)
      (`MaterialInstanceDynamic.SetScalarParameterValue` (`self.LeftPlatform_MID`) "EmissiveStrength" _0_10)
      (`MaterialInstanceDynamic.SetScalarParameterValue` (`self.RightPlatform_MID`) "EmissiveStrength" _0_10))))

(event `self.ReceiveBeginPlay`
  ;[1 1 1] Begin Play - Create our 3 Dynamic Materials for our platforms and set collision to ignore on the middle
  (bind _returnvalue (`PrimitiveComponent.CreateDynamicMaterialInstance` (`self.Platform`) 0 "/Game/Blueprints/Platforms/Mat_Platform_Finish.Mat_Platform_Finish"))
  (set `self.MiddlePlatform_MID` _returnvalue)
  (bind _returnvalue_2 (`PrimitiveComponent.CreateDynamicMaterialInstance` (`self.StaticMesh`) 0 "/Game/Blueprints/Platforms/Mat_SolidEmissive_Yellow.Mat_SolidEmissive_Yellow"))
  (set `self.LeftPlatform_MID` _returnvalue_2)
  (bind _returnvalue_3 (`PrimitiveComponent.CreateDynamicMaterialInstance` (`self.StaticMesh1`) 0 "/Game/Blueprints/Platforms/Mat_SolidEmissive_Yellow.Mat_SolidEmissive_Yellow"))
  (set `self.RightPlatform_MID` _returnvalue_3)
  (`PrimitiveComponent.SetCollisionResponseToChannel` (`self.Platform`) "ECC_Visibility" "ECR_Ignore"))

(fn `UserConstructionScript`)