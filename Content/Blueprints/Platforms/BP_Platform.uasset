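; Clickable platform actor that starts hidden and reports clicks to the game mode, with a one-second timer blocking repeat clicks.
; Hovering plays a timeline that pulses the emissive strength of its dynamic material.
; ToggleVisibility sets visibility and Visibility-channel collision to control clickability.
; Cheating overrides can force it visible or leave visibility untouched while clickability still toggles.
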(event `self.ReceiveBeginPlay`
  ;[1 1 1] Turn ourselves off on Begin Play and create our Material Instance so we can pulse
  (`self.ToggleVisibility` false)
  (bind _returnvalue (`PrimitiveComponent.CreateDynamicMaterialInstance` (`self.Platform`) 0 "/Game/Blueprints/Platforms/Mat_Platform.Mat_Platform"))
  (set `self.MaterialInstRef` _returnvalue))

(event `PulseMaterial`
  ;[1 1 1] Pulse the Material
  (bind (_direction _0_10) (`Timeline|0-0.5` :!via `PlayFromStart`)
    (:`Update`
      (`MaterialInstanceDynamic.SetScalarParameterValue` (`self.MaterialInstRef`) "EmissiveStrength" _0_10))))

(event `self.Platform.OnClicked`
  (params (TouchedComponent :type "PrimitiveComponent Object Reference") (ButtonPressed :type "Key Structure" :default "AnyKey"))
  ;[1 1 1] Handle being clicked on
  (if (not (`self.WasClickedOn`))
    (set `self.WasClickedOn` true)
    (message `/Game/Blueprints/Framework/BPI_LevelGameMode.PlatformClickedOn` (`GameplayStatics.GetGameMode`) self) ; Tell our Game Mode we were clicked on
    (`KismetSystemLibrary.K2_SetTimer` null "ResetWasClickedOn" 1.0) ; Allow ourself to be clicked on again in a second
  ))

(event `ResetWasClickedOn`
  ;[1 1 1] Allow ourself to be clicked on again
  (set `self.WasClickedOn` false))

(event `/Game/Blueprints/Platforms/BPI_Platform.ToggleVisibility`
  (params (IsVisible :type Boolean) (CheatingTurnedOn :type Boolean))
  ;[1 1 1] Handle Toggling the Visibility
  (if CheatingTurnedOn
    (`SceneComponent.SetVisibility` (`self.Root`) true true) ; We need to be visible so turn ourselves visible
    (else
      (if (not (`/Game/Blueprints/Framework/BP_Jam_GameInstance.IsCheating` (cast `/Game/Blueprints/Framework/BP_Jam_GameInstance` (`GameplayStatics.GetGameInstance`) :!pure true)))
        (`SceneComponent.SetVisibility` (`self.Root`) IsVisible true) ; Toggle Visibility
      )
      (`PrimitiveComponent.SetCollisionResponseToChannel` (`self.Platform`) "ECC_Visibility" (select `bool` IsVisible :`false` "ECR_Ignore" :`true` "ECR_Block" :!type "ECollisionResponse Enum")) ; Turn off the ability to click on us
    )))

(event `self.Platform.OnBeginCursorOver`
  (params (TouchedComponent :type "PrimitiveComponent Object Reference"))
  ;[1 1 1] Pulse the material when we mouse over it
  (`self.PulseMaterial`))

(fn `UserConstructionScript`)