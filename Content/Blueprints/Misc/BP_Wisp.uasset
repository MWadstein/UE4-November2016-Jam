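; BP_Wisp is an actor that sends a wisp particle effect along a path of referenced platform actors.
; The construction script rebuilds its spline with a point slightly above each PlatformPath entry.
; ActivateWisp spawns the emitter at the first point, and Tick moves it along the spline by elapsed time over WispLifetime.
; At the end of the path, it destroys the emitter and itself.
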(event `self.ReceiveTick`
  (params (DeltaSeconds :type "Float (single-precision)"))
  (bind _returnvalue (/ (`self.DurationOfWisp`) (`self.WispLifetime`)))
  ;[1 1 1] Move our Wisp if we need to move
  (if (`self.WispIsMoving`)
    (set `self.DurationOfWisp` (+ DeltaSeconds (`self.DurationOfWisp`))) ; Increment how long we have been moving for
    (`SceneComponent.K2_SetWorldLocation` (`self.WispEmitter`) (`SplineComponent.GetLocationAtTime` (`self.Spline`) _returnvalue "World" false) false false) ; Set our location on the spline based on how long we have been alive and how long we want to be alive
    (if (>= _returnvalue 1.0)
      (set `self.WispIsMoving` false) ; Stop our Wisp
      (`ActorComponent.K2_DestroyComponent` (`self.WispEmitter`)) ; Detroy our Emitter
      (`self.K2_DestroyActor`) ; Destroy the Wisp
    )))

(event `ActivateWisp`
  ;[1 1 1] Turn on our Wisp
  (bind _returnvalue (`GameplayStatics.SpawnEmitterAtLocation` "/Game/Particle/Part_Wisp.Part_Wisp" (`SplineComponent.GetLocationAtSplinePoint` (`self.Spline`) 0 "World") (struct) false)) ; Spawn our Emitter
  (set `self.WispEmitter` _returnvalue)
  (set `self.WispIsMoving` true))

(fn `UserConstructionScript`
  (`SplineComponent.ClearSplinePoints` (`self.Spline`) true)
  (for _array_element (`self.PlatformPath`)
    (bind (_returnvalue_x _returnvalue_y _returnvalue_z) (`KismetMathLibrary.BreakVector` (`SceneComponent.K2_GetComponentLocation` (`/Game/Blueprints/Platforms/BP_Platform.Root` _array_element))))
    (`SplineComponent.AddSplinePoint` (`self.Spline`) (`KismetMathLibrary.MakeVector` _returnvalue_x _returnvalue_y (+ _returnvalue_z 25.0)) "World" true)))