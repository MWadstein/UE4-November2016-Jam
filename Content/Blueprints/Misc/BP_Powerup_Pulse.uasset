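; Pulse multiplier pickup that shows its value as "x" text and applies it when a character hits it.
; BeginPlay writes MultiplierValue, rounded to a whole number, to the TextRender.
; A Sphere hit by any BPI_Jam_Character implementer plays a 2D sound and particle burst, overwrites PulseMultiplier on BP_Jam_LevelGameMode, then destroys the pickup.
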(event `self.ReceiveBeginPlay`
  ;[1 1 1] Assign our Multiplier Variable to the Text Renderer
  (`TextRenderComponent.K2_SetText` (`self.TextRender`) (`KismetTextLibrary.Conv_StringToText` (`KismetStringLibrary.Concat_StrStr` "x" (`KismetTextLibrary.Conv_TextToString` (`KismetTextLibrary.Conv_DoubleToText` (`self.MultiplierValue`) "HalfToEven" true 1 324 0 0))))))

(event `self.Sphere.OnComponentHit`
  (params (HitComponent :type "PrimitiveComponent Object Reference") (OtherActor :type "Actor Object Reference") (OtherComp :type "PrimitiveComponent Object Reference") (NormalImpulse :type "Vector Structure") (Hit :type "HitResult Structure (by ref)"))
  ;[1 1 1] The player hit us so adjust their Pulse Multiplier in the Game Mode
  (if (`KismetSystemLibrary.DoesImplementInterface` OtherActor "/Game/Blueprints/Character/BPI_Jam_Character.BPI_Jam_Character_C")
    (`GameplayStatics.PlaySound2D` "/Game/Audio/Sounds/Powerup_Pickup_Cue.Powerup_Pickup_Cue") ; Play a Sound
    (bind _returnvalue (`GameplayStatics.SpawnEmitterAtLocation` "/Game/Particle/Part_Powerup.Part_Powerup" (`SceneComponent.K2_GetComponentLocation` (`self.Sphere`)))) ; Spawn a pickup effect
    (`ActorComponent.Activate` _returnvalue true) ; Turn on the pickup effect
    (set `/Game/Blueprints/Framework/BP_Jam_LevelGameMode.PulseMultiplier` (`self.MultiplierValue`) (cast `/Game/Blueprints/Framework/BP_Jam_LevelGameMode` (`GameplayStatics.GetGameMode`) :!pure true)) ; Tell our Game Mode our new Multiplier
    (`self.K2_DestroyActor`) ; Destroy Ourself
  ))

(fn `UserConstructionScript`)