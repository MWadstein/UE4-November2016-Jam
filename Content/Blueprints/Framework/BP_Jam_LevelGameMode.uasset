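; Level game mode for a turn-limited puzzle in which the player clicks to hop between platforms toward a finish.
; A sphere trace around the pawn refreshes which platforms are visible on pulses and moves, toggled through messages.
; Each regular hop teleports the pawn and spends a turn from BP_LevelSetup's allowance, then updates UI and checks win/lose.
; It also handles music and end screens; an older timeline-based movement graph is left disconnected.
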(event `/Game/Blueprints/Framework/BPI_LevelGameMode.ToggleMusic`
  (params (PlayMusic :type Boolean))
  ;[1 1 1] Handle Toggling the Music
  (if PlayMusic
    (`/Engine/EditorBlueprintResources/StandardMacros.IsValid` (`self.AudioCompMusic`) ; Do we have an audio component already for this?
      (:`Is Not Valid`
        (bind _returnvalue (`GameplayStatics.CreateSound2D` "/Game/Audio/Music/MusicLoop_Cue.MusicLoop_Cue")) ; Create our Sound Component
        (bind _output_get (set `self.AudioCompMusic` _returnvalue))
        (`AudioComponent.Play` _output_get 0.0) ; Play our Music
      ))
    (else
      (`/Engine/EditorBlueprintResources/StandardMacros.IsValid` (`self.AudioCompMusic`) ; Do we have an audio component already for this?
        (:`Is Valid`
          (`AudioComponent.Stop` (`self.AudioCompMusic`)) ; Stop the Music
          (set `self.AudioCompMusic` null) ; Invalidate our Audio Component
        )))))

(event `/Game/Blueprints/Framework/BPI_LevelGameMode.FinishClickedOn`
  (params (Platform :type "/Game/Blueprints/Platforms/BP_Platform_Finish Object Reference"))
  ;[1 1 1] Handle clicking on the Finish Platform
  (for _array_element (`self.VisiblePlatformArray`)
    (if (== (`.HitActor` (`GameplayStatics.BreakHitResult` _array_element)) Platform)
      (`self.K2_SetActorTransform` (`Controller.K2_GetPawn` (`GameplayStatics.GetPlayerController` 0)) (`self.GetAdjustedtNewLocation` (`/Game/Blueprints/Platforms/BP_Platform_Finish.Root` Platform)) false false) ; Set our Player to the New Platform
      (`KismetSystemLibrary.Delay` 2.0) ; Wait a few seconds
      (set `self.PlayerReachedFinish` true)
      (`self.CheckForWinOrLose`) ; Check if we won or lost
    )))

(event `/Game/Blueprints/Framework/BPI_LevelGameMode.PulseThePlayer`
  (params (Radius :type "Float (single-precision)"))
  ;[1 1 1] Pulse Visibility of the Surrounding Platforms
  (`self.PulseVisibility` Radius))

(event `self.ReceiveBeginPlay`
  ;[1 1 1] Initialization Stuff
  (`self.LoadSettingsForTheLevel`) ; Load our Settings
  (bind _returnvalue (`|CreateWidget` "/Game/Blueprints/UI/UMG_GameUI.UMG_GameUI_C")) ; Create our Game UI
  (bind _output_get (set `self.GameUIRef` _returnvalue))
  (`UserWidget.AddToViewport` _output_get 0) ; Add it to the screen
  (`self.UpdateTheUI`) ; Make sure our UI is current
  (set `PlayerController.bShowMouseCursor` true (`GameplayStatics.GetPlayerController` 0)))

(event `/Game/Blueprints/Framework/BPI_LevelGameMode.PlatformClickedOn`
  (params (CurrentTarget :type "/Game/Blueprints/Platforms/BP_Platform Object Reference"))
  ;[1 1 1] Move our Character to the new Platform
  (`self.K2_SetActorTransform` (`Controller.K2_GetPawn` (`GameplayStatics.GetPlayerController` 0)) (`self.GetAdjustedtNewLocation` (`/Game/Blueprints/Platforms/BP_Platform.Root` CurrentTarget)) false true) ; Set our Character to the location of the platform + 33 on the Z
  (`/Engine/EditorBlueprintResources/StandardMacros.DecrementInt` (`self.TurnsLeft`) ; Remove a Turn
    (:`  `
      (for _array_element (`self.VisiblePlatformArray`)
        (message `/Game/Blueprints/Platforms/BPI_Platform.ToggleVisibility` (`.HitActor` (`GameplayStatics.BreakHitResult` _array_element)) false false) ; Hide all our current visible platforms
      )
      (bind _outhits (`self.SetVisiblePlatforms` (`self.BasePulseRadius`))) ; Fiond and Set our Platforms that will become visibile
      (set `self.VisiblePlatformArray` _outhits)
      (for _array_element_2 (`self.VisiblePlatformArray`)
        (message `/Game/Blueprints/Platforms/BPI_Platform.ToggleVisibility` (`.HitActor` (`GameplayStatics.BreakHitResult` _array_element_2)) true false) ; Turn on any platforms near us
      )
      (`self.CheckForWinOrLose`) ; Check for Win or Lose
    )))

(fn `CheckForWinOrLose`
  (bind _returnvalue (`GameplayStatics.GetPlayerController` 0))
  (bind _returnvalue_2 (`GameplayStatics.GetPlayerController` 0))
  (`self.UpdateTheUI`)
  (if (<= (`self.TurnsLeft`) 0)
    (message `/Game/Blueprints/Character/BPI_Jam_Character.KillPlayer` (`Controller.K2_GetPawn` (`GameplayStatics.GetPlayerController` 0)))
    (`self.ToggleMusic` false)
    (`GameplayStatics.PlaySound2D` "/Game/Audio/Sounds/Lose_Cue.Lose_Cue")
    (bind _returnvalue_3 (`|CreateWidget` "/Game/Blueprints/UI/UMG_GameOver.UMG_GameOver_C"))
    (`UserWidget.AddToViewport` _returnvalue_3 0)
    (`self.DisableInput` (`Controller.K2_GetPawn` _returnvalue_2) _returnvalue_2)
    (elif (`self.PlayerReachedFinish`)
      (`self.ToggleMusic` false)
      (`GameplayStatics.PlaySound2D` "/Game/Audio/Sounds/Win_Cue.Win_Cue")
      (bind _returnvalue_4 (`|CreateWidget` "/Game/Blueprints/UI/UMG_YouWin.UMG_YouWin_C"))
      (`UserWidget.AddToViewport` _returnvalue_4 0)
      (`self.DisableInput` (`Controller.K2_GetPawn` _returnvalue) _returnvalue))))

(fn `LoadSettingsForTheLevel`
  (bind _outactors (`GameplayStatics.GetAllActorsOfClass` "/Game/Blueprints/Framework/BP_LevelSetup.BP_LevelSetup_C")) ; Get our Set up BP from the level
  (bind _output_get (set `self.AllowedTurns` (`/Game/Blueprints/Framework/BP_LevelSetup.AllowedTurns` (`KismetArrayLibrary.Array_Get` _outactors)))) ; How many Turns?
  (set `self.TurnsLeft` _output_get))

(fn `PulseVisibility`
  (params (Distance :type "Float (double-precision)"))
  (bind _outhits (`self.SetVisiblePlatforms` Distance)) ; Find and SEt our platforms that will become visible
  (set `self.VisiblePlatformArray` _outhits)
  (for _array_element (`self.VisiblePlatformArray`)
    (message `/Game/Blueprints/Platforms/BPI_Platform.ToggleVisibility` (`.HitActor` (`GameplayStatics.BreakHitResult` _array_element)) true false) ; Make them visible
  ))

(fn `UpdateTheUI`
  (bind _gameuiref (`self.GameUIRef`))
  (bind _gameuiref_2 (`self.GameUIRef`))
  (`/Game/Blueprints/UI/UMG_GameUI.SetTurnsLeft` _gameuiref (`self.TurnsLeft`)) ; Show how many turns left
  (`/Game/Blueprints/UI/UMG_GameUI.SetPlayerName` _gameuiref (`/Game/Blueprints/Framework/BP_Jam_GameInstance.PlayerName` (cast `/Game/Blueprints/Framework/BP_Jam_GameInstance` (`GameplayStatics.GetGameInstance`) :!pure true))) ; Set our players Name
  (`UserWidget.PlayAnimation` _gameuiref_2 (`/Game/Blueprints/UI/UMG_GameUI.ShakeTurnsLeft` _gameuiref_2) 0.0 1 "Forward" 1.0) ; Play an animation when the player moves showing the new turns left
)

(fn `UserConstructionScript`)