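; Player character for a jam game that provides orbit camera control and handles its own death.
; BeginPlay sets an initial camera pitch, and two axis inputs drive controller pitch and yaw to look around the character.
; KillPlayer spawns a lose particle effect, waits briefly, then destroys the actor.
; The Destroyed handler is disabled, and leftover game mode turn-check and name-label logic never runs.
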(event `self.ReceiveDestroyed`
  ;[1 1 1] DISABLED - Causes problem with reset.  Should not need anymore due to having Reset and Fixing Movement
)

(event `self.ReceiveBeginPlay`
  ;[1 1 1] Set our initial Camera Pitch to above the player
  (`self.AddControllerPitchInput` 15.0))

(event `InputAxis|CameraPitch`
  (params (AxisValue :type "Float (single-precision)"))
  ;[1 1 1] Allow Mouse Look Up/Down
  (`self.AddControllerPitchInput` AxisValue))

(event `InputAxis|CameraRotation`
  (params (AxisValue :type "Float (single-precision)"))
  ;[1 1 1] Rotate the Camera around the Character
  (`self.AddControllerYawInput` AxisValue))

(event `/Game/Blueprints/Character/BPI_Jam_Character.KillPlayer`
  ;[1 1 1] Handle the player being killed
  (`GameplayStatics.SpawnEmitterAtLocation` "/Game/Particle/Part_Lose.Part_Lose" (`self.K2_GetActorLocation`)) ; Spawn our death emitter
  (`KismetSystemLibrary.Delay` 0.5)
  (`self.K2_DestroyActor`) ; Kill our Player
)

(fn `UserConstructionScript`)