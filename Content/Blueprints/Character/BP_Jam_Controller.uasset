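; Player controller that toggles a simple pause menu from the PauseMenu input action or the TogglePauseMenu event.
; Opening creates UMG_SimplePauseMenu, disables input on the controlled pawn and drops global time dilation to near zero instead of truly pausing.
; Closing removes and clears the widget reference, re-enables pawn input and restores normal time.
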(event `/Game/Blueprints/Character/BPI_Jam_Controller.TogglePauseMenu`
  (bind _returnvalue (`GameplayStatics.GetPlayerController` 0))
  (bind _returnvalue_2 (`GameplayStatics.GetPlayerController` 0))
  ;[1 1 1] Handle the Pause Button Interaction.  Also handle the Widget passing the Close event back to the player
  (`/Engine/EditorBlueprintResources/StandardMacros.IsValid` (`self.PauseMenuRef`) :!label _label ; Is our Widget Valid?
    (:`Is Valid`
      (`Widget.RemoveFromParent` (`self.PauseMenuRef`)) ; Remove our Widget from the Viewport
      ;;[1 1 1] Handle Enabling the input to the camera and character and removing the mouse cursor
      (`self.EnableInput` (`self.K2_GetPawn` _returnvalue) _returnvalue)
      (set `self.PauseMenuRef` null) ; Destroy our reference to our Widget as we no longer need it
      (`GameplayStatics.SetGlobalTimeDilation` 1.0))
    (:`Is Not Valid`
      (bind _returnvalue_3 (`|CreateWidget` "/Game/Blueprints/UI/UMG_SimplePauseMenu.UMG_SimplePauseMenu_C")) ; Create a New Widget
      (bind _output_get (set `self.PauseMenuRef` _returnvalue_3)) ; Store a Reference to our Widget
      ;;[1 1 1] Handle Disabling the player input to the camera and character and allowing mouse input
      (`UserWidget.AddToViewport` _output_get 0) ; Add to our Viewport
      (`self.DisableInput` (`self.K2_GetPawn` _returnvalue_2) _returnvalue_2)
      (`GameplayStatics.SetGlobalTimeDilation` 0.001))))

(event `InputAction|PauseMenu`
  (params (Key :type "Key Structure" :default "AnyKey"))
  ;[1 1 1] Handle the Pause Button Interaction.  Also handle the Widget passing the Close event back to the player
  (:`Pressed`
    (goto _label)))

(fn `UserConstructionScript`)